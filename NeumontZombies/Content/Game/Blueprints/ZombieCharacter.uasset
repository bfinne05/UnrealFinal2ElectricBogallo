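; Zombie enemy character that the player shoots for score and that can attack the player.
; Overlap with an actor tagged "Bulllet" (triple-l spelling) adds score to the first-person player and destroys the zombie in one hit.
; AttackPlayer starts the attack montage, then subtracts clamped Health from the player after a fixed delay, with no range or hit check.
; The event has no caller in this Blueprint.
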(event Custom|AttackPlayer
  (Animation|Montage|PlayMontage (Variables|Character|GetMesh) "/Game/Game/Models/Animation/Zombie_Attack__1__mixamo_com_Montage.Zombie_Attack__1__mixamo_com_Montage"
    (:then
      (bind _asbp_first_person_character (Utilities|Casting|CastToBP_FirstPersonCharacter (Game|GetPlayerCharacter 0)))
      (Utilities|FlowControl|Delay 1.2)
      (Variables|/Game/FirstPerson/Blueprints/BP_FirstPersonCharacter.BP_FirstPersonCharacter_C|SetHealth _asbp_first_person_character (Math|Float|Clamp(Float) (- (Variables|/Game/FirstPerson/Blueprints/BP_FirstPersonCharacter.BP_FirstPersonCharacter_C|GetHealth _asbp_first_person_character) 1e+01) 0.0 1e+02)))))

(event EventBeginPlay)

(event Collision|EventActorBeginOverlap
  (params (OtherActor :type Actor%20Object%20Reference))
  (if (Actor|ActorHasTag OtherActor "Bulllet")
    (bind _asbp_first_person_character (Utilities|Casting|CastToBP_FirstPersonCharacter (Game|GetPlayerCharacter 0)))
    (Variables|/Game/FirstPerson/Blueprints/BP_FirstPersonCharacter.BP_FirstPersonCharacter_C|SetScore _asbp_first_person_character (+ (Variables|/Game/FirstPerson/Blueprints/BP_FirstPersonCharacter.BP_FirstPersonCharacter_C|GetScore _asbp_first_person_character) 50))
    (Actor|DestroyActor)))

(event EventTick
  (params (DeltaSeconds :type Float%20%28single-precision%29)))

(fn ConstructionScript)